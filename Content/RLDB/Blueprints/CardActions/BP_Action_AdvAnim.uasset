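; BP_Action_AdvAnim is a card action that animates a Puppet actor and holds the action sequence until that animation reports back.
; PlayAction sends the Animation message to the Puppet both before and after binding to its BP_PuppetComponent's animation event.
; CheckAnimationEvent waits for the event matching Animation, then unbinds and calls EndAction so the next action can proceed.
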(event `self.PlayAction`
  ;[0 0 0] Attempts to animate the input Puppet actor. Waits for the Puppet to call the appropriate animation event (as set in Animation) before proceeding to the next action
  (message `/Game/RLDB/Blueprints/Interfaces/BPI_CardPuppet.AnimatePuppet` (`self.Puppet`) (`self.Animation`))
  (add `/Game/RLDB/Blueprints/Core/BP_PuppetComponent.OnAnimationEvent` (`self.GetComponentByClass` (`self.Puppet`) "/Game/RLDB/Blueprints/Core/BP_PuppetComponent.BP_PuppetComponent_C") (delegate `CheckAnimationEvent`))
  (message `/Game/RLDB/Blueprints/Interfaces/BPI_CardPuppet.AnimatePuppet` (`self.Puppet`) (`self.Animation`)))

(event `CheckAnimationEvent`
  (params (Puppet :type "Actor Object Reference") (Animation :type "GameplayTag Structure"))
  ;[0 0 0] Attempts to animate the input Puppet actor. Waits for the Puppet to call the appropriate animation event (as set in Animation) before proceeding to the next action
  (if (== Animation (`self.Animation`))
    (remove `/Game/RLDB/Blueprints/Core/BP_PuppetComponent.OnAnimationEvent` (`self.GetComponentByClass` (`self.Puppet`) "/Game/RLDB/Blueprints/Core/BP_PuppetComponent.BP_PuppetComponent_C") (delegate `CheckAnimationEvent`))
    (`self.EndAction`)))

(fn `UserConstructionScript`
  (`parent.UserConstructionScript`))