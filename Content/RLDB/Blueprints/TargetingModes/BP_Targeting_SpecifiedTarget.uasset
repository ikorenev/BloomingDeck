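; Targeting mode for card effects that resolves targets from a list of already specified targets.
; FindValidTargets keeps each valid entry whose gameplay tag component exactly matches at least one of the card effect's gameplay tags.
; It returns the filtered list, while its TargetsFound output is always false.
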(fn `FindValidTargets`
  (params (SpecifiedTargets :type "Array of Actor Object Reference (by ref)") (CardEffect :type "/Game/RLDB/Blueprints/Structs/FCardEffect Structure") (Card :type "/Game/RLDB/Blueprints/Core/BP_Card Object Reference") (bPreview :type Boolean))
  (returns (bTargetsFound :type Boolean) (ValidTargets :type "Array of Actor Object Reference"))
  (locals (LocalValidTargets :type "Array of Actor Object Reference"))
  (for _array_element SpecifiedTargets
    (if (`KismetSystemLibrary.IsValid` _array_element)
      (if (`BlueprintGameplayTagLibrary.HasAnyTags` (`/Game/RLDB/Blueprints/Libraries/BPFL_CardEffect.GetEffectGameplayTags` (`local.CardEffect`)) (`/Game/RLDB/Blueprints/Core/BP_GameplayTagComponent.GameplayTags` (`Actor.GetComponentByClass` _array_element "/Game/RLDB/Blueprints/Core/BP_GameplayTagComponent.BP_GameplayTagComponent_C")) true)
        (`KismetArrayLibrary.Array_Add` (`local.LocalValidTargets`) _array_element))))
  (return false (`local.LocalValidTargets`)))