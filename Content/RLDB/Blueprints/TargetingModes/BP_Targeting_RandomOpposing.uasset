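; Card targeting mode that picks one random minion on the track opposing the card.
; FindValidTargets gathers all minions on the opposing track and reports failure when none exist.
; In preview it returns every candidate, so all possible targets show; otherwise it returns a single randomly chosen minion.
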(fn `FindValidTargets`
  (params (SpecifiedTargets :type "Array of Actor Object Reference (by ref)") (CardEffect :type "/Game/RLDB/Blueprints/Structs/FCardEffect Structure") (Card :type "/Game/RLDB/Blueprints/Core/BP_Card Object Reference") (bPreview :type Boolean))
  (returns (bTargetsFound :type Boolean) (ValidTargets :type "Array of Actor Object Reference"))
  (locals (LocalValidTargets :type "Array of Actor Object Reference"))
  (bind (_bfoundanytargets _minions) (`self.GetAllMinionsOnOpposingTrack` Card))
  (if _bfoundanytargets
    (set `local.LocalValidTargets` _minions)
    (if (`local.bPreview`)
      (return true (`local.LocalValidTargets`))
      (else
        (return true (`|MakeArray` (`KismetArrayLibrary.Array_Random` (`local.LocalValidTargets`))))))
    (else
      (return false))))