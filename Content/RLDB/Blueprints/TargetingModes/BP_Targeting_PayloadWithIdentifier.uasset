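; BP_Targeting_PayloadWithIdentifier is a card effect targeting mode that targets an actor previously stored as a payload on the card player.
; It looks up the player's payload holder component using the effect's Identifier and returns the value as the sole target if it is an Actor, otherwise finding none.
; The payload is destroyed on access unless the effect carries the exact Flag.DoNotClear gameplay tag.
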(fn `FindValidTargets`
  (params (SpecifiedTargets :type "Array of Actor Object Reference (by ref)") (CardEffect :type "/Game/RLDB/Blueprints/Structs/FCardEffect Structure") (Card :type "/Game/RLDB/Blueprints/Core/BP_Card Object Reference") (bPreview :type Boolean))
  (returns (bTargetsFound :type Boolean) (ValidTargets :type "Array of Actor Object Reference"))
  (bind ((`GameplayTags_24_CC3A96B84AC557056996C8A91DF06498` _gameplaytags) (`Identifier_40_EB9B02FD45D3654F82EBB2BAC1AD9613` _identifier)) (break `/Game/RLDB/Blueprints/Structs/FCardEffect` CardEffect))
  (bind _cardplayer (`/Game/RLDB/Blueprints/Libraries/BPFL_Singletons.GetCardPlayer`))
  (bind (_bsuccess _value) (`/Game/RLDB/Blueprints/Core/BP_PayloadHolderComponent.AccessPayload` (`/Game/RLDB/Blueprints/Core/BP_CardPlayer.BP_PayloadHolderComponent` _cardplayer) _identifier (not (`BlueprintGameplayTagLibrary.HasTag` _gameplaytags (struct :`TagName` "Flag.DoNotClear") true))))
  (if _bsuccess
    (bind _asactor (cast `Actor` _value)
      (:`then`
        (return true (`|MakeArray` _asactor)))
      (:`CastFailed`
        _)))
  (return false))