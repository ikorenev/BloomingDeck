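; Card effect that summons minions onto the minion track of the minion that owns the parent card.
; ResolveCardEffect looks up the minion row in a data table, then adds it once per EffectValue, at least once, flagged as spawned during gameplay.
; A Position.Back gameplay tag inserts behind the back minion; otherwise summons go to the front at index zero.
; It fails if the owner is not a minion or the row is missing.
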(fn `ResolveCardEffect`
  (params (TargetActor :type "Actor Object Reference"))
  (returns (bSuccess :type Boolean))
  (bind (_useddata_datatable _useddata_rowname) (break `DataTableRowHandle` (`self.UsedData`)))
  (bind _asbp_minion (cast `/Game/RLDB/Blueprints/Core/BP_Minion` (`Actor.GetOwner` (`self.ParentCard`)))
    (:`then`
      (bind _returnvalue (`|GetDataTableRow` _useddata_datatable _useddata_rowname)
        (:`then`
          (for _ (range (+ (`KismetMathLibrary.Max` (- (`self.EffectValue`) 1)) 1))
            (bind _miniontrack (`/Game/RLDB/Blueprints/Core/BP_Minion.MinionTrack` _asbp_minion))
            (`/Game/RLDB/Blueprints/Core/BP_MinionTrack.AddMinionToTrack` _miniontrack (`KismetMathLibrary.SelectInt` (+ (`.BackIndex` (`/Game/RLDB/Blueprints/Core/BP_MinionTrack.GetBackMinion` _miniontrack)) 1) 0 (`BlueprintGameplayTagLibrary.HasTag` (`self.GameplayTags`) (struct :`TagName` "Position.Back") true)) _returnvalue true))
          (return true))
        (:`RowNotFound`
          (return false))))
    (:`CastFailed`
      (return false))))