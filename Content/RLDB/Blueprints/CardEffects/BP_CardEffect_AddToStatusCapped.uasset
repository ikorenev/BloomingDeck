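; Card effect that adds its EffectValue to a status on the target actor without pushing that status past its maximum.
; When the target already has the TargetComponent status and it is Maxable, the amount is trimmed to the room left below MaxValue.
; Otherwise the full value is sent through AddToStatusMessage, with the effect as payload.
; Resolution fails only if TargetComponent is not a BP_Status.
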(fn `ResolveCardEffect`
  (params (TargetActor :type "Actor Object Reference"))
  (returns (bSuccess :type Boolean))
  (bind _returnvalue (`Actor.GetComponentByClass` TargetActor (`self.TargetComponent`)))
  (bind _asbp_status (cast `/Game/RLDB/Blueprints/Statuses/BP_Status` _returnvalue :!pure true))
  (bind _statusvalue (`/Game/RLDB/Blueprints/Statuses/BP_Status.StatusValue` _asbp_status))
  (bind _asbp_status_2 (castclass `/Game/RLDB/Blueprints/Statuses/BP_Status` (`self.TargetComponent`))
    (:`then`
      (if (`KismetSystemLibrary.IsValid` _returnvalue)
        (if (`/Game/RLDB/Blueprints/Statuses/BP_Status.bMaxable` _asbp_status)
          (message `/Game/RLDB/Blueprints/Interfaces/BPI_CardTarget.AddToStatus` (`local.TargetActor`) _asbp_status_2 (- (`KismetMathLibrary.Min` (`/Game/RLDB/Blueprints/Statuses/BP_Status.MaxValue` _asbp_status) (+ (`self.EffectValue`) _statusvalue)) _statusvalue) true self)
          (return true)
          (else
            _)))
      (message `/Game/RLDB/Blueprints/Interfaces/BPI_CardTarget.AddToStatus` (`local.TargetActor`) _asbp_status_2 (`self.EffectValue`) true self)
      (return true))
    (:`CastFailed`
      (return false))))