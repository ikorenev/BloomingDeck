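; Card effect that adds an existing target card, or one spawned from a data table row, to a player card pile, defaulting to the hand.
; Spawned cards are owned by the parent card's owner or tagged main hero; without minions, OwnerID becomes the first persistent hero.
; It repeats the add by EffectValue, firing a card-generate event each time, with an optional slow-display flag.
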(fn `ResolveCardEffect`
  (params (TargetActor :type "Actor Object Reference"))
  (returns (bSuccess :type Boolean))
  (locals (LocalTargetPileClass :type "/Game/RLDB/Blueprints/Piles/BP_PileComponent Object Reference") (LocalCard :type "/Game/RLDB/Blueprints/Core/BP_Card Object Reference"))
  (bind _localcard (`local.LocalCard`))
  (bind _useddata_datatable (break `DataTableRowHandle` (`self.UsedData`)))
  ;[0 0 0] Takes either a card reference, or if none is available a reference to a card in a data table, and attempts to add to the specified pile. Required input: TargetComponent (Pile to add to), Either Target (Card) for an existing card or UsedData (Card data table row) to add a new card, Effect Value (Numer of cards to add). Optional input: Flag.Slow (for displaying the card for longer before it moves to the pile)
  (bind _asbp_card (cast `/Game/RLDB/Blueprints/Core/BP_Card` TargetActor)
    (:`then`
      (set `local.LocalCard` _asbp_card))
    (:`CastFailed`
      (if (`KismetSystemLibrary.IsValid` _useddata_datatable)
        (bind (_bsuccess _mainhero) (message `/Game/RLDB/Blueprints/Interfaces/BPI_CardGameInstance.GetMainHero` (`GameplayStatics.GetGameInstance`)))
        (bind _returnvalue (`|SpawnActorFromClass` "/Game/RLDB/Blueprints/Core/BP_Card.BP_Card_C" (`KismetMathLibrary.MakeTransform` (0.0 0.0 0.0)) "AlwaysSpawn" "OverrideRootScale" (select `bool` (`BlueprintGameplayTagLibrary.HasTag` (`self.GameplayTags`) (struct :`TagName` "Target.Hero") true) :`false` (`Actor.GetOwner` (`self.ParentCard`)) :`true` _mainhero) (`/Game/RLDB/Blueprints/Libraries/BPFL_Card.MakeCardStructFromCardData` (`self.UsedData`)) null))
        (set `local.LocalCard` _returnvalue)
        (else
          (return false)))))
  (if (> (`self.EffectValue`) 0)
    (bind _returnvalue_2 (`GameplayStatics.GetActorOfClass` "/Game/RLDB/Blueprints/Core/BP_Minion.BP_Minion_C"))
    (if (not (`KismetSystemLibrary.IsValid` _returnvalue_2))
      (bind _persistentheroes (message `/Game/RLDB/Blueprints/Interfaces/BPI_CardGameInstance.GetPersistentHeroesFromInstance` (`GameplayStatics.GetGameInstance`)))
      (setmembers `/Game/RLDB/Blueprints/Structs/FCard` :`StructRef` (`/Game/RLDB/Blueprints/Core/BP_Card.CardDataDeck` (`local.LocalCard`)) :`OwnerID` (`.UniqueID_53_2854C97C4349924C1E5F7B922ADBA3AE` (break `/Game/RLDB/Blueprints/Structs/FMinion` (`|GetArrayItem` _persistentheroes)))))
    (bind _asbp_pile_component (castclass `/Game/RLDB/Blueprints/Piles/BP_PileComponent` (`self.TargetComponent`)) ; If no pile is specified, adds to hand
      (:`then`
        (set `local.LocalTargetPileClass` _asbp_pile_component))
      (:`CastFailed`
        (set `local.LocalTargetPileClass` "/Game/RLDB/Blueprints/Piles/BP_PileComponent_Hand.BP_PileComponent_Hand_C")))
    (for _ (range 1 (+ (`self.EffectValue`) 1))
      (message `/Game/RLDB/Blueprints/Interfaces/BPI_Pile.AttemptAddExistingCard` (`Actor.GetComponentByClass` (`/Game/RLDB/Blueprints/Libraries/BPFL_Singletons.GetCardPlayerPure`) (`local.LocalTargetPileClass`)) (`local.LocalCard`))
      (`/Game/RLDB/Blueprints/Core/BP_DispatcherHubComponent.CallEventWithCallTags` (`/Game/RLDB/Blueprints/Core/BP_Card.BP_DispatcherHubComponent_Local` _localcard) (struct :`TagName` "Event.Card.Generate") _localcard null "NewEnumerator2" (select `bool` (`BlueprintGameplayTagLibrary.HasTag` (`self.GameplayTags`) (struct :`TagName` "Flag.Slow") true) :`true` (struct :`GameplayTags` (struct :`(TagName` "Flag.Slow"))) :!type "GameplayTagContainer Structure")))
    (return true)
    (else
      (return false))))