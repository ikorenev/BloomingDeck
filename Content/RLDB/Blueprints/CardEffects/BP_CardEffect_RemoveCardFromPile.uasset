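; Card effect that removes a targeted card from one of the card player's piles.
; It casts the target to a card and the configured target component to a pile component class, then finds that component on the player and requests removal.
; On success it refreshes that pile's card count in the player UI by pile tag and returns true; failed casts or requests return false.
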(fn `ResolveCardEffect`
  (params (TargetActor :type "Actor Object Reference"))
  (returns (bSuccess :type Boolean))
  (bind _asbp_card (cast `/Game/RLDB/Blueprints/Core/BP_Card` TargetActor)
    (:`then`
      (bind _asbp_pile_component (castclass `/Game/RLDB/Blueprints/Piles/BP_PileComponent` (`self.TargetComponent`))
        (:`then`
          (bind _returnvalue (`Actor.GetComponentByClass` (`/Game/RLDB/Blueprints/Libraries/BPFL_Singletons.GetCardPlayerPure`) _asbp_pile_component))
          (bind _bsuccess (`/Game/RLDB/Blueprints/Piles/BP_PileComponent.RequestRemoveCardFromPile` _returnvalue _asbp_card))
          (if _bsuccess
            (bind _cardplayer (`/Game/RLDB/Blueprints/Libraries/BPFL_Singletons.GetCardPlayer`))
            (`/Game/RLDB/Widgets/WBP_Layout_RLDB.UpdatePileWidgetAmount` (`/Game/RLDB/Blueprints/Core/BP_CardPlayer.PlayerUI` _cardplayer) (`/Game/RLDB/Blueprints/Piles/BP_PileComponent.PileTag` _returnvalue) (`KismetArrayLibrary.Array_Length` (`/Game/RLDB/Blueprints/Piles/BP_PileComponent.Cards` _returnvalue)))
            (return true)
            (else
              (return false))))
        (:`CastFailed`
          (return false))))
    (:`CastFailed`
      (return false))))