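; Card effect that draws a specific target card into the card player's hand.
; When EffectValue is positive, it casts the target actor to a card and passes it to the hand pile's DrawCard, failing if the cast fails.
; The source pile is the target component if that is a pile, otherwise the draw pile.
; A non-positive EffectValue succeeds without drawing.
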(fn `ResolveCardEffect`
  (params (TargetActor :type "Actor Object Reference"))
  (returns (bSuccess :type Boolean))
  (bind _returnvalue (`Actor.GetComponentByClass` (`/Game/RLDB/Blueprints/Libraries/BPFL_Singletons.GetCardPlayerPure`) "/Game/RLDB/Blueprints/Piles/BP_PileComponent_Hand.BP_PileComponent_Hand_C"))
  (if (> (`self.EffectValue`) 0)
    (bind _asbp_card (cast `/Game/RLDB/Blueprints/Core/BP_Card` TargetActor)
      (:`then`
        (bind _asbp_pile_component (castclass `/Game/RLDB/Blueprints/Piles/BP_PileComponent` (`self.TargetComponent`))
          (:`then`
            (`/Game/RLDB/Blueprints/Piles/BP_PileComponent_Hand.DrawCard` _returnvalue _asbp_card _asbp_pile_component))
          (:`CastFailed`
            (`/Game/RLDB/Blueprints/Piles/BP_PileComponent_Hand.DrawCard` _returnvalue _asbp_card "/Game/RLDB/Blueprints/Piles/BP_PileComponent_Draw.BP_PileComponent_Draw_C")))
        (return true))
      (:`CastFailed`
        (return false)))
    (else
      (return true))))