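; Card use rule that makes playing a card cost an amount of one of the card player's statuses.
; The check looks up the status component by the class in the rule data and allows use only if its value covers the cost.
; An insufficient value returns a "Not Enough" message with the status name, while a missing status fails with no message.
; Resolving the rule subtracts the cost from that status on the player.
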(fn `CheckIfUseAllowed`
  (params (UseRuleData :type "/Game/RLDB/Blueprints/Structs/FUseRule Structure"))
  (returns (bAllowed :type Boolean) (FailMessage :type String))
  (bind ((`Status_5_80417C034BA8BB613212268821F8F45E` _status) (`Cost_8_0CA3B59A490140FA38B3D9B52A204217` _cost)) (break `/Game/RLDB/Blueprints/Structs/FUseRule` UseRuleData))
  (bind _cardplayer (`/Game/RLDB/Blueprints/Libraries/BPFL_Singletons.GetCardPlayer`))
  (bind _returnvalue (`Actor.GetComponentByClass` _cardplayer _status))
  (if (`KismetSystemLibrary.IsValid` _returnvalue)
    (if (>= (`/Game/RLDB/Blueprints/Statuses/BP_Status.StatusValue` _returnvalue) _cost)
      (return true "")
      (else
        (return false (`KismetStringLibrary.Concat_StrStr` "Not Enough " (`KismetTextLibrary.Conv_TextToString` (`/Game/RLDB/Blueprints/Statuses/BP_Status.FriendlyName` _returnvalue))))))
    (else
      (return false ""))))

(fn `ResolveUseConsequence`
  (params (UseRuleData :type "/Game/RLDB/Blueprints/Structs/FUseRule Structure"))
  (returns (bSuccess :type Boolean))
  (bind ((`Status_5_80417C034BA8BB613212268821F8F45E` _status) (`Cost_8_0CA3B59A490140FA38B3D9B52A204217` _cost)) (break `/Game/RLDB/Blueprints/Structs/FUseRule` UseRuleData))
  (bind _cardplayer (`/Game/RLDB/Blueprints/Libraries/BPFL_Singletons.GetCardPlayer`))
  (message `/Game/RLDB/Blueprints/Interfaces/BPI_CardTarget.SubtractFromStatus` _cardplayer _status _cost true null)
  (return true))