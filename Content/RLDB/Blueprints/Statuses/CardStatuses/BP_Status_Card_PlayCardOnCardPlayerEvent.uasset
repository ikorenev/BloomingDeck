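; Card status that automatically plays its card when one of a configurable set of card player events fires while the card is in hand.
; Entering the hand binds those tags to the card player's dispatcher hub and opens a gate; the exit-hand event unbinds and closes it.
; Events passing the gate queue delays and an AutoPlay event around an untargeted use that skips playability checks and consequences.
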(event `self.ReceiveBeginPlay`
  (`parent.ReceiveBeginPlay`)
  (`/Game/RLDB/Blueprints/Core/BP_DispatcherHubComponent.BindMultipleEventsToHub` (`.ReturnValue` (`self.GetOwnersDispatcherHub`)) self (struct :`GameplayTags` (struct :`(TagName` "Event.Card.EnterHand") :`(TagName` "Event.Card.ExitHand")))))

(event `/Game/RLDB/Blueprints/Interfaces/BPI_EventHolder.RunEvent`
  (params (EventTag :type "GameplayTag Structure") (CallingObject :type "Object Object Reference (by ref)") (bGlobal :type Boolean) (Payload :type "Object Object Reference (by ref)") (CallTags :type "GameplayTagContainer Structure (by ref)"))
  (`|SwitchGameplayTag` EventTag
    (:`Default`
      (`/Engine/EditorBlueprintResources/StandardMacros.Gate` true :!label _label
        (:`Exit`
          (bind _asbp_card (cast `/Game/RLDB/Blueprints/Core/BP_Card` (`self.GetOwner`)))
          (`/Game/RLDB/Blueprints/Libraries/BPFL_Singletons.QueueDelay` 0.4)
          (`/Game/RLDB/Blueprints/Libraries/BPFL_Singletons.QueueEventInGlobalDispatcherHub` (struct :`TagName` "Event.Action.AutoPlay") (`self.GetOwner`) null 1.0)
          (`/Game/RLDB/Blueprints/Core/BP_Card.AttemptUseCardUntargeted` _asbp_card true true true)
          (`/Game/RLDB/Blueprints/Libraries/BPFL_Singletons.QueueDelay` 1.0))))
    (:`Event.Card.EnterHand`
      (`|ExecutionSequence`
        (:`then_0`
          (`/Game/RLDB/Blueprints/Core/BP_DispatcherHubComponent.BindMultipleEventsToHub` (`/Game/RLDB/Blueprints/Core/BP_CardPlayer.BP_DispatcherHubComponent_Local` (`/Game/RLDB/Blueprints/Libraries/BPFL_Singletons.GetCardPlayerPure`)) self (`self.GameplayTags`)))
        (:`then_1`
          (goto _label :!via `Open`))))
    (:`Event.Card.ExitHand`
      (`|ExecutionSequence`
        (:`then_0`
          (`/Game/RLDB/Blueprints/Core/BP_DispatcherHubComponent.UnbindMultipleEventsFromHub` (`/Game/RLDB/Blueprints/Core/BP_CardPlayer.BP_DispatcherHubComponent_Local` (`/Game/RLDB/Blueprints/Libraries/BPFL_Singletons.GetCardPlayerPure`)) self (`self.GameplayTags`)))
        (:`then_1`
          (goto _label :!via `Close`))))))