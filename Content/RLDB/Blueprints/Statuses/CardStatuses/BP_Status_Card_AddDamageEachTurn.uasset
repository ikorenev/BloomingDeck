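; Card status that raises its owning card's attack effect values at each turn end while the card is in hand.
; It binds to the card's event hub and the player's TurnEnd event, with a gate opened and closed by entering and leaving the hand.
; Each gated turn end adds StatusValue to a running total, which is reapplied when the card enters hand or receives a modify-in-hand event.
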(event `self.ReceiveBeginPlay`
  (`parent.ReceiveBeginPlay`)
  (bind _asbp_card (cast `/Game/RLDB/Blueprints/Core/BP_Card` (`self.GetOwner`)))
  (bind _output_get (set `self.OwningCard` _asbp_card))
  (`/Game/RLDB/Blueprints/Core/BP_DispatcherHubComponent.BindMultipleEventsToHub` (`/Game/RLDB/Blueprints/Core/BP_Card.BP_DispatcherHubComponent_Local` _output_get) self (struct :`GameplayTags` (struct :`(TagName` "Event.Card.ModifyInHand") :`(TagName` "Event.Card.EnterHand") :`(TagName` "Event.Card.ExitHand"))))
  (bind _cardplayer (`/Game/RLDB/Blueprints/Libraries/BPFL_Singletons.GetCardPlayer`))
  (`/Game/RLDB/Blueprints/Core/BP_DispatcherHubComponent.BindEventToHub` (`/Game/RLDB/Blueprints/Core/BP_CardPlayer.BP_DispatcherHubComponent_Local` _cardplayer) self (struct :`TagName` "Event.TurnEnd")))

(event `/Game/RLDB/Blueprints/Interfaces/BPI_EventHolder.RunEvent`
  (params (EventTag :type "GameplayTag Structure") (CallingObject :type "Object Object Reference (by ref)") (bGlobal :type Boolean) (Payload :type "Object Object Reference (by ref)") (CallTags :type "GameplayTagContainer Structure (by ref)"))
  (`|SwitchGameplayTag` EventTag
    (:`Event.TurnEnd`
      (`/Engine/EditorBlueprintResources/StandardMacros.Gate` true :!label _label
        (:`Exit`
          (set `self.CurrentModification` (+ (`self.CurrentModification`) (`self.StatusValue`)))
          (`/Game/RLDB/Blueprints/Core/BP_Card.ModifyCardEffectValues` :`self` (`self.OwningCard`) :`Modification` (`self.StatusValue`) :`RequiredTags` (struct :`GameplayTags` (struct :`(TagName` "Effect.Attack")))))))
    (:`Event.Card.EnterHand`
      (`|ExecutionSequence`
        (:`then_0`
          (goto _label :!via `Open`))
        (:`then_1`
          (`/Game/RLDB/Blueprints/Core/BP_Card.ModifyCardEffectValues` :`self` (`self.OwningCard`) :`Modification` (`self.CurrentModification`) :`RequiredTags` (struct :`GameplayTags` (struct :`(TagName` "Effect.Attack"))) :!label _label_2))))
    (:`Event.Card.ExitHand`
      (goto _label :!via `Close`))
    (:`Event.Card.ModifyInHand`
      (goto _label_2))))