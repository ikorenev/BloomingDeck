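; A card status component that shifts the Mana cost of its owning card until that card exits the hand.
; On begin play it binds to the card's exit-hand event and adds its status value to the stat cost, clamped at zero.
; It notifies the card when the cost is set, reapplies on modify-in-hand events, and destroys itself on exit.
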(event `self.ReceiveBeginPlay`
  (`parent.ReceiveBeginPlay`)
  (bind _asbp_card (cast `/Game/RLDB/Blueprints/Core/BP_Card` (`self.GetOwner`)))
  (bind _output_get (set `self.OwningCard` _asbp_card))
  (`/Game/RLDB/Blueprints/Core/BP_Card.BindLocalCardEvents` _output_get self (struct :`GameplayTags` (struct :`(TagName` "Event.Card.ExitHand") :`(TagName` "Event.Card.ModifyInHand"))))
  (`self.ModifyCost`))

(event `ModifyCost`
  (bind (_bvalid _statuscost) (`/Game/RLDB/Blueprints/Core/BP_Card.GetStatusCostValueFromUseRules` (`self.OwningCard`) "NewEnumerator0" "/Game/RLDB/Blueprints/Statuses/BP_Status_Mana.BP_Status_Mana_C"))
  (bind _bsuccess (`/Game/RLDB/Blueprints/Core/BP_Card.SetUseRuleCost` (`self.OwningCard`) "/Game/RLDB/Blueprints/CardUseRules/BP_UseRule_StatCost.BP_UseRule_StatCost_C" "/Game/RLDB/Blueprints/Statuses/BP_Status_Mana.BP_Status_Mana_C" (`KismetMathLibrary.Max` (+ _statuscost (`self.StatusValue`))) "NewEnumerator0" false))
  (if _bsuccess
    (`/Game/RLDB/Blueprints/Core/BP_Card.OnThisCardModified` (`self.OwningCard`))))

(event `/Game/RLDB/Blueprints/Interfaces/BPI_EventHolder.RunEvent`
  (params (EventTag :type "GameplayTag Structure") (CallingObject :type "Object Object Reference (by ref)") (bGlobal :type Boolean) (Payload :type "Object Object Reference (by ref)") (CallTags :type "GameplayTagContainer Structure (by ref)"))
  (if (== CallingObject (`self.OwningCard`))
    (`|SwitchGameplayTag` EventTag
      (:`Event.Card.ModifyInHand`
        (`self.ModifyCost`))
      (:`Event.Card.ExitHand`
        (`self.K2_DestroyComponent`)))))