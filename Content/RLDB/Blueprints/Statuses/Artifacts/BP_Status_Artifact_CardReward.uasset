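; Artifact status that holds a pending card reward and grants it to the main hero when interacted with.
; When value is added, it stores reward data from the card effect payload, falling back to a default, until a valid table is set.
; Interact spawns a "GainCard" card, injects that data into its add-new-card-to-pile effect, auto-plays it, then removes the status.
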(fn `AddStatusValue`
  (params (Amount :type Integer) (bShowSplashNumber :type Boolean) (bShowSplashIcon :type Boolean) (bRefreshAppearance :type Boolean) (Payload :type "Object Object Reference"))
  (returns (NewValue :type Integer))
  (bind _cardrewarddata_datatable (break `DataTableRowHandle` (`self.CardRewardData`)))
  (bind _newvalue (`parent.AddStatusValue` Amount bShowSplashNumber bShowSplashIcon bRefreshAppearance Payload))
  (if (not (`KismetSystemLibrary.IsValid` _cardrewarddata_datatable))
    (bind _asbp_card_effect (cast `/Game/RLDB/Blueprints/CardEffects/BP_CardEffect` (`local.Payload`))
      (:`then`
        (bind _useddata (`/Game/RLDB/Blueprints/CardEffects/BP_CardEffect.UsedData` _asbp_card_effect))
        (set `self.CardRewardData` (select `bool` (`KismetSystemLibrary.IsValid` (`.DataTable` (break `DataTableRowHandle` _useddata))) :`false` (`self.DefaultRewardData`) :`true` _useddata))
        (return _newvalue))
      (:`CastFailed`
        _)))
  (return _newvalue))

(fn `Interact`
  (params (Tags :type "GameplayTagContainer Structure"))
  (returns (bSuccess :type Boolean))
  (locals (LocalCardEffects :type "Array of /Game/RLDB/Blueprints/Structs/FCardEffect Structure"))
  (`|SwitchGameplayTagContainer` Tags
    (:`(GameplayTags=((TagName="StatusBar.RewardBar")))`
      (bind (_bsuccess _mainhero) (message `/Game/RLDB/Blueprints/Interfaces/BPI_CardGameInstance.GetMainHero` (`GameplayStatics.GetGameInstance`)))
      (bind _returnvalue (`|SpawnActorFromClass` "/Game/RLDB/Blueprints/Core/BP_Card.BP_Card_C" (`KismetMathLibrary.MakeTransform` (0.0 0.0 0.0)) "AlwaysSpawn" "OverrideRootScale" _mainhero (`/Game/RLDB/Blueprints/Libraries/BPFL_Card.MakeCardStructFromCardData` (make `DataTableRowHandle` "/Game/RLDB/Data/Cards/DT_Cards_Rewards.DT_Cards_Rewards" "GainCard")) null))
      (bind _output_get (set `local.LocalCardEffects` (`/Game/RLDB/Blueprints/Core/BP_Card.GetCardEffects` _returnvalue "NewEnumerator0")))
      (for (_array_element _array_index) _output_get
        (if (== (`.EffectClass_12_BB4B6E404EF340B02CA017B3DE840E2D` (break `/Game/RLDB/Blueprints/Structs/FCardEffect` _array_element)) "/Game/RLDB/Blueprints/CardEffects/BP_CardEffect_AddNewCardToPile.BP_CardEffect_AddNewCardToPile_C")
          (bind _structout (setmembers `/Game/RLDB/Blueprints/Structs/FCardEffect` :`StructRef` _array_element :`UsedData` (`self.CardRewardData`)))
          (`KismetArrayLibrary.Array_Set` (`local.LocalCardEffects`) _array_index _structout)))
      (`/Game/RLDB/Blueprints/Core/BP_Card.SetCardEffects` _returnvalue "NewEnumerator0" (`local.LocalCardEffects`))
      (bind _bsuccess_2 (`/Game/RLDB/Blueprints/Core/BP_Card.AttemptUseCardUntargeted` _returnvalue false false true))
      (`self.RemoveStatus`)
      (return _bsuccess_2))))