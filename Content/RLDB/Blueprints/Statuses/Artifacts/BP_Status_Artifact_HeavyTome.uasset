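; BP_Status_Artifact_HeavyTome is an artifact status that trades card draw for mana gain.
; It overrides AddStatusValue, calling the parent and then continuing only when the owner is a BP_CardPlayer.
; It silently sends the owner a ManaGain increase equal to the change in status value and a Draw reduction of a flat 1 per call, regardless of amount.
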(fn `AddStatusValue`
  (params (Amount :type Integer) (bShowSplashNumber :type Boolean) (bShowSplashIcon :type Boolean) (bRefreshAppearance :type Boolean) (Payload :type "Object Object Reference"))
  (returns (NewValue :type Integer))
  (locals (LocalOldValue :type Integer :default 0))
  (bind _returnvalue (`self.GetOwner`))
  (set `local.LocalOldValue` (`self.StatusValue`))
  (bind _newvalue (`parent.AddStatusValue` Amount bShowSplashNumber bShowSplashIcon bRefreshAppearance Payload))
  (cast `/Game/RLDB/Blueprints/Core/BP_CardPlayer` _returnvalue)
  (message `/Game/RLDB/Blueprints/Interfaces/BPI_CardTarget.AddToStatus` _returnvalue "/Game/RLDB/Blueprints/Statuses/BP_Status_ManaGain.BP_Status_ManaGain_C" (- _newvalue (`local.LocalOldValue`)) false null)
  (message `/Game/RLDB/Blueprints/Interfaces/BPI_CardTarget.SubtractFromStatus` (`self.GetOwner`) "/Game/RLDB/Blueprints/Statuses/BP_Status_Draw.BP_Status_Draw_C" 1 false null)
  (return _newvalue))