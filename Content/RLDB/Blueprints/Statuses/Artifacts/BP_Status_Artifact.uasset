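; BP_Status_Artifact is a status component for artifacts, which belong to the card player and are recorded in the game instance.
; On a hero minion, it removes itself at BeginPlay, first passing its value to the card player if the instance lacks that artifact.
; Interacting grants it to the player and hides the reward icon.
; Added value is saved to the instance, unless the player passes itself as payload to prevent duplication.
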(event `self.ReceiveBeginPlay`
  (cast `/Game/RLDB/Blueprints/Core/BP_CardPlayer` (`self.GetOwner`)
    (:`then`
      (`parent.ReceiveBeginPlay`))
    (:`CastFailed`
      (bind _asbp_minion (cast `/Game/RLDB/Blueprints/Core/BP_Minion` (`self.GetOwner`))
        (:`then`
          (if (`BlueprintGameplayTagLibrary.HasTag` (`/Game/RLDB/Blueprints/Core/BP_Minion.GetGameplayTags` _asbp_minion) (struct :`TagName` "Target.Hero") true)
            (bind _bhasartifact (message `/Game/RLDB/Blueprints/Interfaces/BPI_CardGameInstance.CheckIfInstanceHasArtifact` (`GameplayStatics.GetGameInstance`) (`GameplayStatics.GetObjectClass` self)))
            (if (not _bhasartifact)
              (bind _cardplayer (`/Game/RLDB/Blueprints/Libraries/BPFL_Singletons.GetCardPlayer`))
              (`/Game/RLDB/Blueprints/Interfaces/BPI_CardTarget.AddToStatus` _cardplayer (`GameplayStatics.GetObjectClass` self) (`self.StatusValue`) false null))
            (`self.K2_DestroyComponent`)
            (else
              (`parent.ReceiveBeginPlay`))))
        (:`CastFailed`
          (`parent.ReceiveBeginPlay`))))))

(fn `AddStatusValue`
  (params (Amount :type Integer) (bShowSplashNumber :type Boolean) (bShowSplashIcon :type Boolean) (bRefreshAppearance :type Boolean) (Payload :type "Object Object Reference"))
  (returns (NewValue :type Integer))
  (bind _asbp_card_player (cast `/Game/RLDB/Blueprints/Core/BP_CardPlayer` (`self.GetOwner`))
    (:`then`
      (if (!= _asbp_card_player Payload)
        (message `/Game/RLDB/Blueprints/Interfaces/BPI_CardGameInstance.AddArtifactToInstance` (`GameplayStatics.GetGameInstance`) (make `/Game/RLDB/Blueprints/Structs/FStatus` (`GameplayStatics.GetObjectClass` self) (`local.Amount`) (`self.GameplayTags`)))
        (bind _newvalue (`parent.AddStatusValue` (`local.Amount`) (`local.bShowSplashNumber`) (`local.bShowSplashIcon`) (`local.bRefreshAppearance`) (`local.Payload`)))
        (return _newvalue)
        (else
          _)))
    (:`CastFailed`
      _))
  (bind _newvalue_2 (`parent.AddStatusValue` (`local.Amount`) (`local.bShowSplashNumber`) (`local.bShowSplashIcon`) (`local.bRefreshAppearance`) (`local.Payload`)))
  (return _newvalue_2))

(fn `Interact`
  (params (Tags :type "GameplayTagContainer Structure"))
  (returns (bSuccess :type Boolean))
  (`|SwitchGameplayTagContainer` Tags
    (:`(GameplayTags=((TagName="StatusBar.RewardBar")))`
      (bind _cardplayer (`/Game/RLDB/Blueprints/Libraries/BPFL_Singletons.GetCardPlayer`))
      (`/Game/RLDB/Blueprints/Core/BP_CardPlayer.AddToStatus` _cardplayer (`GameplayStatics.GetObjectClass` self) (`self.StatusValue`) true null)
      (`|SpawnActorFromClass` "/Game/RLDB/Blueprints/CardActions/BP_Action_ModifyStatus.BP_Action_ModifyStatus_C" (`KismetMathLibrary.MakeTransform` (0.0 0.0 0.0)) "AlwaysSpawn" "OverrideRootScale" null self 0 false false "" true "HideReward" false -1.0 null) ; HideReward fed as text override causes the status icon to not collapse the status icon,\npreventing the rewards from shuffling over when selected
      (return true))))