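; Pile component for a card game that acts as a destroy pile, removing any cards that land in it.
; On Tick, a non-empty Cards array triggers a DoOnce that destroys every card actor and empties the array.
; The DoOnce resets after ResetDelay, spacing out successive purges.
; ClearPile does no work and always returns false.
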(event `self.ReceiveTick`
  (params (DeltaSeconds :type "Float (single-precision)"))
  (if (> (`KismetArrayLibrary.Array_Length` (`self.Cards`)) 0)
    (`/Engine/EditorBlueprintResources/StandardMacros.DoOnce` false :!label _label
      (:`Completed`
        (for _array_element (`self.Cards`)
          (`Actor.K2_DestroyActor` _array_element))
        (`KismetArrayLibrary.Array_Clear` (`self.Cards`))
        (`KismetSystemLibrary.Delay` (`self.ResetDelay`))
        (goto _label :!via `Reset`)))))

(fn `ClearPile`
  (returns (bSuccess :type Boolean))
  (return false))